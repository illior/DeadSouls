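; BP_Character is a player character Blueprint that limits camera pitch and offers a debug control for game speed.
; On BeginPlay it casts its controller to PlayerController and clamps the camera manager's view pitch to a symmetric range.
; PageUp and PageDown step global time dilation up or down, and Tick prints the current value on screen under a fixed key.
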(event EventTick
  (params (DeltaSeconds :type Float%20%28single-precision%29))
  (Development|PrintString (Utilities|String|ToString(Float) (Class|GameplayStatics|GetGlobalTimeDilation)) true false "(R=0.000000,G=0.000000,B=0.000000,A=1.000000)" 2.0 "323123"))

(event EventBeginPlay
  (bind _asplayer_controller (Utilities|Casting|CastToPlayerController (Pawn|GetController)))
  (Variables|/Script/Engine.PlayerCameraManager|SetViewPitchMin (Variables|/Script/Engine.PlayerController|GetPlayerCameraManager _asplayer_controller) -6e+01)
  (Variables|/Script/Engine.PlayerCameraManager|SetViewPitchMax (Variables|/Script/Engine.PlayerController|GetPlayerCameraManager _asplayer_controller) 6e+01))

(event Input|KeyboardEvents|PageDown
  (params (Key :type Key%20Structure :default "None"))
  (:Pressed
    (Utilities|Time|SetGlobalTimeDilation (+ (Class|GameplayStatics|GetGlobalTimeDilation) -0.1))))

(event Input|KeyboardEvents|PageUp
  (params (Key :type Key%20Structure :default "None"))
  (:Pressed
    (Utilities|Time|SetGlobalTimeDilation (+ (Class|GameplayStatics|GetGlobalTimeDilation) 0.1))))

(fn ConstructionScript)
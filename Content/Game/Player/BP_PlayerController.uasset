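; Player controller Blueprint that owns the inventory screen.
; On BeginPlay it creates WBP_Inventory, adds it to the viewport and keeps it collapsed.
; The IA_OpenInventory input calls PauseGame and reveals the widget, while the CloseInventory event collapses it again without any unpause call.
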(event Custom|CloseInventory
  (Widget|SetVisibility (Variables|Default|GetInventoryWidget) "Collapsed"))

(event Input|EnhancedActionEvents|EnhancedInputActionIA_OpenInventory
  (params (ActionValue :type Boolean) (ElapsedSeconds :type Float%20%28double-precision%29) (TriggeredSeconds :type Float%20%28double-precision%29) (InputAction :type Input%20Action%20Object%20Reference :default "/Game/Game/Player/Input/Default/IA_OpenInventory.IA_OpenInventory"))
  (:Started
    (Class|DSPlayerController|PauseGame)
    (Widget|SetVisibility (Variables|Default|GetInventoryWidget) "SelfHitTestInvisible")))

(event EventBeginPlay
  (bind _returnvalue (UserInterface|CreateWidget "/Game/Game/UI/Inventory/WBP_Inventory.WBP_Inventory_C" self))
  (bind _output_get (Variables|Default|SetInventoryWidget _returnvalue))
  (UserInterface|Viewport|AddtoViewport _output_get 0)
  (Widget|SetVisibility _output_get "Collapsed"))

(fn ConstructionScript)
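; BP_BaseAddItem is a base interactable pickup actor that offers an item to the character's inventory.
; Interacting passes its TestItem to the character's InventoryComponent through TryAddNewItem.
; It listens to the item's OnItemUpdated event and destroys itself once the item's outer is no longer this actor or its count reaches zero.
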(event OnItemUpdated(TestItem)
  (params (InItemData :type DS%20Item%20Data%20Object%20Reference))
  (if (or (!= (Utilities|GetOuterObject InItemData) self) (== (Variables|/Script/InventorySystem.DSItemData|GetCount InItemData) 0))
    (Actor|DestroyActor)))

(event EventInteract
  (Class|DSInventoryComponent|TryAddNewItem (Variables|/Script/DeadSouls.DSCharacter|GetInventoryComponent (Variables|Default|GetCharacter)) (Variables|DeadSouls:Interaction|GetTestItem)))

(fn ConstructionScript)